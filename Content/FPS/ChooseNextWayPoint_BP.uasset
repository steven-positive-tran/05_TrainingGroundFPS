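; Behavior tree task that advances an AI-controlled ThirdPersonCharacter along its patrol route.
; It reads the pawn's PatrolPoints array and writes the entry at the blackboard Index to the WayPoint key.
; It then increments Index, wrapping by array length with modulo so the route loops, and finishes with success.
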(event EventReceiveExecuteAI
  (params (OwnerController :type AI%20Controller%20Object%20Reference) (ControlledPawn :type Pawn%20Object%20Reference))
  ;[1 1 1] Get Patrol Points
  (CallFunction|GetPatrolPoints ControlledPawn)
  ;[1 1 1] SetWayPoint
  (bind _returnvalue (CallFunction|SetWayPoint))
  ;[1 1 1] Cycle Index
  (CallFunction|CycleIndex _returnvalue)
  (AI|BehaviorTree|FinishExecute true))

(fn GetPatrolPoints
  (params (Object :type Object%20Object%20Reference))
  (bind _asthird_person_character (Utilities|Casting|CastToThirdPersonCharacter Object))
  (Variables|Default|SetPatrol%20Points (Variables|/Game/ThirdPersonCPP/Blueprints/ThirdPersonCharacter.ThirdPersonCharacter_C|GetPatrolPoints _asthird_person_character)))

(fn SetWayPoint
  (bind _index (Variables|Default|GetIndex))
  (bind _returnvalue (Class|BTFunctionLibrary|GetBlackboardValueasInt _index))
  (Class|BTFunctionLibrary|SetBlackboardValueasObject (Variables|Default|GetWayPoint) (Utilities|Array|Get(acopy) (Variables|Default|GetPatrol%20Points) _returnvalue))
  (return _returnvalue))

(fn CycleIndex
  (params (A :type Integer))
  (Class|BTFunctionLibrary|SetBlackboardValueasInt (Variables|Default|GetIndex) (Math|Integer|%(Integer) (+ A 1) (Utilities|Array|Length (Variables|Default|GetPatrol%20Points)))))